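; BP_FarmHouse is a farmhouse prop that acts as a temporary hiding place for farmers, releasing them again after a delay.
; SetFarmerSpawnTimer increments an occupancy count and starts a timer using FarmerHideTime.
; On expiry, RespawnFarmer spawns a BP_Farmer at an offset from the house, decrements occupancy and chains further timers while occupants remain.
; A debug key triggers the same spawn logic directly.
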(event Custom|SetFarmerSpawnTimer
  (Math|Integer|IncrementInt (Variables|Default|GetOccupancy)
    (:%20%20
      (Utilities|Time|SetTimerbyEvent (delegate Custom|RespawnFarmer) (Variables|Default|GetFarmerHideTime)))))

(event Custom|RespawnFarmer
  (Game|SpawnActorfromClass "/Game/NPC/FarmerNPC/BP_Farmer.BP_Farmer_C" (Math|Transform|MakeTransform (+ (Transformation|GetActorLocation) "100.000000,0.000000,50.000000") "0, 0, 0" "1.000000,1.000000,1.000000") "AdjustIfPossibleButAlwaysSpawn" "MultiplyWithRoot" 0 0)
  (bind _result (Math|Integer|DecrementInt (Variables|Default|GetOccupancy))
    (:%20%20
      (if (> _result 0)
        (Utilities|Time|SetTimerbyEvent (delegate Custom|ContinueSpawningFarmers) (Variables|Default|GetFarmerHideTime))))))

(event Custom|ContinueSpawningFarmers
  (CallFunction|RespawnFarmer))

(event Input|KeyboardEvents|DebugKey7
  (params (Key :type Key%20Structure :default "None") (ActionValue :type Input%20Action%20Value%20Structure))
  (:Pressed
    (Game|SpawnActorfromClass "/Game/NPC/FarmerNPC/BP_Farmer.BP_Farmer_C" (Math|Transform|MakeTransform (+ (Transformation|GetActorLocation) "100.000000,0.000000,50.000000") "0, 0, 0" "1.000000,1.000000,1.000000") "AdjustIfPossibleButAlwaysSpawn" "MultiplyWithRoot" 0 0)
    (bind _result (Math|Integer|DecrementInt (Variables|Default|GetOccupancy))
      (:%20%20
        (if (> _result 0)
          (Utilities|Time|SetTimerbyEvent (delegate Custom|ContinueSpawningFarmers) (Variables|Default|GetFarmerHideTime)))))))

(fn ConstructionScript)